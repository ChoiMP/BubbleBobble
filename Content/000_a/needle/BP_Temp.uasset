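; BP_Temp is a gauge actor whose mesh rotates like a needle to show TempValue from BubbleGameInstance.
; BeginPlay snaps the mesh's relative yaw to the value, remapped through a clamped range and offset to center the sweep.
; Tick eases the yaw toward the current value with RInterpTo, using a slightly narrower sweep than the initial snap.
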(event EventBeginPlay
  (bind _asbubble_game_instance (Utilities|Casting|CastToBubbleGameInstance (Game|GetGameInstance)))
  (Transformation|SetRelativeRotation (Variables|Default|GetSM_MERGED_Temp_Cube_283) (Math|Rotator|MakeRotator 0.0 0.0 (- (Math|Float|MapRangeClamped (Math|Conversions|ToFloat(Integer) (Variables|/Game/BubbleGameInstance.BubbleGameInstance_C|GetTempValue _asbubble_game_instance)) 0.0 1e+02 0.0 2.8e+02) 1.4e+02)) false false))

(event Collision|EventActorBeginOverlap
  (params (OtherActor :type Actor%20Object%20Reference)))

(event EventTick
  (params (DeltaSeconds :type Float%20%28single-precision%29))
  (bind _sm_merged_temp_cube_283 (Variables|Default|GetSM_MERGED_Temp_Cube_283))
  (bind _asbubble_game_instance (Utilities|Casting|CastToBubbleGameInstance (Game|GetGameInstance)))
  (Transformation|SetRelativeRotation _sm_merged_temp_cube_283 (Math|Interpolation|RInterpTo (Variables|/Script/Engine.SceneComponent|GetRelativeRotation _sm_merged_temp_cube_283) (Math|Rotator|MakeRotator 0.0 0.0 (- (Math|Float|MapRangeClamped (Math|Conversions|ToFloat(Integer) (Variables|/Game/BubbleGameInstance.BubbleGameInstance_C|GetTempValue _asbubble_game_instance)) 0.0 1e+02 0.0 2.7e+02) 135.0)) (Utilities|Time|GetWorldDeltaSeconds) 3.0) false false))

(fn ConstructionScript)