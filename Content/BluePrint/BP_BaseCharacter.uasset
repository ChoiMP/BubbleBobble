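; Base character for a bubble card game, managing a deck, hand and board display of remaining elemental bubbles.
; After a BeginPlay delay, Setting spawns Fire, Water, Bubble and Wind cards from DeckData and builds type-grouped sprite icons on Board.
; Drawing refills an empty Hand with up to three cards, teleporting them to spawn points for Player-tagged characters.
; OnUseBubble locates an icon via per-type counts, dims it and removes it from tracking.
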(event Custom|OnDrawBubble
  ;[0.15 0.15 0.15 0.5] Picking less than 3 cards
  (Utilities|PickingLessthan3)
  (CallFunction|IteratingHandandSpawn))

(event Custom|OnUseBubble
  (params (BubbleType :type BubbleType%20Enum :default "NewEnumerator0"))
  (bind _returnvalue (Math|Conversions|ToInteger(Byte) BubbleType))
  (bind _bubblecount (Variables|Default|GetBubbleCount))
  (bind _output (Utilities|Array|Get(acopy) _bubblecount _returnvalue))
  ;[0.15 0.15 0.15 0.5] Every time called for each 1 card
  (if (> _output 0)
    (Variables|Default|SetIndex 0)
    (for _index (range 0 (- _returnvalue 1))
      (Variables|Default|SetIndex (+ (Utilities|Array|Get(acopy) (Variables|Default|GetBubbleCount) _index) (Variables|Default|GetIndex))))
    (Utilities|IsValid (Utilities|Array|Get(acopy) (Variables|Default|GetBubbles) (Variables|Default|GetIndex))
      (:Is%20Valid
        ;;[0.15 0 0 0.5] [TEMP] 사용했다는 처리(투명, X표시)
        (bind _asbp_bubble (Utilities|Casting|CastToBP_Bubble (Utilities|Array|Get(acopy) (Variables|Default|GetBubbles) (Variables|Default|GetIndex))))
        (Sprite|SetSpriteColor (Variables|/Game/BluePrint/BP_Bubble.BP_Bubble_C|GetPaperSprite _asbp_bubble) "(R=0.200000,G=0.200000,B=0.200000,A=0.500000)")
        (Math|Integer|DecrementInt _output
          (:%20%20
            (Utilities|Array|RemoveIndex (Variables|Default|GetBubbles) (Variables|Default|GetIndex))))))))

(event EventBeginPlay
  (Utilities|FlowControl|Delay 5.0)
  (Utilities|Setting))

(fn ConstructionScript)

(fn DrawBubble
  (bind _deck (Variables|Default|GetDeck))
  (bind _output_get (LocalVariables|SetBubble (Utilities|Array|Get(acopy) _deck)))
  (Utilities|Array|RemoveIndex _deck)
  (Utilities|Array|Add (Variables|Default|GetHand) _output_get)
  (return))

(fn IteratingHandandSpawn
  (if (Actor|ActorHasTag "Player")
    (bind _outactors (Actor|GetAllActorsOfClass "/Game/PlayerCardSpawnPoint.PlayerCardSpawnPoint_C"))
    (for (_array_element _array_index) (Variables|Default|GetHand)
      (bind _returnvalue (Transformation|SetActorLocation _array_element (.location (Transformation|GetActorTransform (Utilities|Array|Get(acopy) _outactors _array_index))) false true))
      (Development|PrintString "Hello"))
    (return)))