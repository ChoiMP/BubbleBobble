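; BP_Pot is a pot Blueprint that tracks two integer gauges, Temperature and Bubble.
; Both gauges reset to zero on BeginPlay.
; AddParameter adds an amount to the gauge chosen by a boolean, clamps it between 0 and 100, then prints both values on screen for debugging.
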(event EventBeginPlay
  (Variables|Default|SetTemperature 0)
  (Variables|Default|SetBubble 0))

(fn ConstructionScript)

(fn AddParameter
  (params (IsTemperature :type Boolean) (Amount :type Integer))
  (if IsTemperature
    (bind _output_get (Variables|Default|SetTemperature (Math|Integer|Clamp(Integer) (+ (Variables|Default|GetTemperature) Amount) 0 100)))
    (else
      (bind _output_get_2 (Variables|Default|SetBubble (Math|Integer|Clamp(Integer) (+ Amount (Variables|Default|GetBubble)) 0 100)))))
  (Development|PrintString (Utilities|String|Append "Temp : " (Utilities|String|ToString(Integer) _output_get) " " "Bubble : " (Utilities|String|ToString(Integer) _output_get_2)))
  (return))