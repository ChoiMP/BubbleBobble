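; BP_Witch is the witch in a turn-based card game, relaying its turn and card-use actions to the BP_BubbleMode game mode.
; Turn start calls DrawCard, an empty temporary stub, and card use, meant to fire after a bubble is used, calls the mode's OnTurnEnd.
; AddParameter forwards an amount and a temperature flag to the mode; its only call here sits in an unconnected chain.
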(event Custom|OnTurnStart
  (CallFunction|DrawCard))

(event Custom|OnUseCard
  ;[0.15 0.15 0.15 0.5] 버블 사용 후 호출
  (bind _asbp_bubble_mode (Utilities|Casting|CastToBP_BubbleMode (Game|GetGameMode)))
  (Default|OnTurnEnd _asbp_bubble_mode))

(fn ConstructionScript)

(fn AddParameter
  (params (IsTemperature :type Boolean) (Amount :type Integer))
  (bind _asbp_bubble_mode (Utilities|Casting|CastToBP_BubbleMode (Game|GetGameMode)))
  (Default|AddParameter _asbp_bubble_mode IsTemperature Amount))

(fn DrawCard
  ;[0.15 0.15 0.15 0.5] [TEMP] 드로우 기능 연동
)