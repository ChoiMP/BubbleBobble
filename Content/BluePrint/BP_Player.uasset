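; BP_Player is a player Blueprint with early scaffolding for using bubbles.
; BeginPlay calls the parent, then prints each BubbleCount entry as debug output.
; OnUseBubble checks the passed actor's exact class against fire, water, bubble and wind bubble types in a chain of branches, none of which has any action yet.
; Tick and overlap events are disabled, and the construction script only calls the parent.
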(event Custom|OnUseBubble
  (params (actor :type Actor%20Object%20Reference))
  (bind _returnvalue (Utilities|GetClass actor))
  (if (not (== _returnvalue "/Game/FireBubble.FireBubble_C"))
    (if (not (== _returnvalue "/Game/WaterBubble.WaterBubble_C"))
      (if (not (== _returnvalue "/Game/BubbleBubble.BubbleBubble_C"))
        (if (== _returnvalue "/Game/WindBubble.WindBubble_C")
          _)))))

(event EventBeginPlay
  (|CallParentFunction)
  (for _array_element (Variables|Default|GetBubbleCount)
    (Development|PrintString (Utilities|String|ToString(Integer) _array_element))))

(event Collision|EventActorBeginOverlap
  (params (OtherActor :type Actor%20Object%20Reference)))

(event EventTick
  (params (DeltaSeconds :type Float%20%28single-precision%29)))

(fn ConstructionScript
  (|CallParentFunction))