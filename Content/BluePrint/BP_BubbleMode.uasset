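; Game mode-style Blueprint for a turn-based card duel between player and enemy witches around a shared pot.
; BeginPlay spawns the pot and both witches, deals cards and starts the player's turn.
; Ending the player's turn flips the turn and draws for both; ending the enemy's currently ends the game through placeholder hand/deck checks.
; Victory requires pot Temperature and Bubble to reach set thresholds, currently zero, and is only printed.
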(event Custom|OnTurnEnd
  ;[0.15 0.15 0.15 0.5] Enemy 턴인가?
  (if (Variables|Default|GetIsPlayerTurn)
    ;[0.15 0.15 0.15 0.5] 턴 종료
    (|EndTurn :!label _label)
    ;[0.15 0.15 0.15 0.5] 드로우
    (CallFunction|DrawCards 3)
    (else
      ;[0.15 0 0 0.502] [TEMP] 핸드가 0 장인가?
      (if true
        ;[0.15 0 0 0.502] [TEMP] 덱이 0장인가?
        (if true
          ;[0.15 0.15 0.15 0.5] 게임 종료
          (CallFunction|CheckVictoryConditions))
        (else
          (goto _label))))))

(event Custom|OnGameEnd
  (params (IsVictory :type Boolean))
  (Development|PrintString (Utilities|String|SelectString "Victory" "Defeat" IsVictory))
  (if IsVictory
    _))

(event EventBeginPlay
  (CallFunction|SetVictoryConditions)
  (CallFunction|SpawnActors)
  (CallFunction|DrawCards 3)
  (Variables|Default|SetIsPlayerTurn true)
  (bind _asbp_witch (Utilities|Casting|CastToBP_Witch (Variables|Default|GetPlayer)))
  (Default|OnTurnStart _asbp_witch))

(fn ConstructionScript)

(fn SetVictoryConditions
  (params (TemperatureCondition :type Integer) (BubbleCondition :type Integer))
  (Variables|Default|SetTemperature%20Condition (Math|Integer|Clamp(Integer) TemperatureCondition 0 100))
  (Variables|Default|SetBubble%20Condition (Math|Integer|Clamp(Integer) BubbleCondition 0 100))
  (return))

(fn CheckVictoryConditions
  (bind _asbp_pot (Utilities|Casting|CastToBP_Pot (Variables|Default|GetPot))
    (:then
      (CallFunction|OnGameEnd (and (>= (Variables|/Game/BluePrint/BP_Pot.BP_Pot_C|GetTemperature _asbp_pot) (Variables|Default|GetTemperature%20Condition)) (>= (Variables|/Game/BluePrint/BP_Pot.BP_Pot_C|GetBubble _asbp_pot) (Variables|Default|GetBubble%20Condition)))))
    (:CastFailed
      (CallFunction|OnGameEnd false))))

(fn AddParameter
  (params (IsTemperature :type Boolean) (Amount :type Integer))
  (bind _asbp_pot (Utilities|Casting|CastToBP_Pot (Variables|Default|GetPot)))
  (Default|AddParameter _asbp_pot IsTemperature Amount)
  (return))

(fn SpawnActors
  (bind _returnvalue (Game|SpawnActorfromClass "/Game/BluePrint/BP_Pot.BP_Pot_C" (Transformation|GetActorTransform) "Undefined" "MultiplyWithRoot" 0 0))
  (Variables|Default|SetPot _returnvalue)
  (bind _returnvalue_2 (Game|SpawnActorfromClass "/Game/BluePrint/BP_Witch.BP_Witch_C" (Transformation|GetActorTransform) "Undefined" "MultiplyWithRoot" 0 0))
  (Variables|Default|SetPlayer _returnvalue_2)
  (bind _returnvalue_3 (Game|SpawnActorfromClass "/Game/BluePrint/BP_Witch.BP_Witch_C" (Transformation|GetActorTransform) "Undefined" "MultiplyWithRoot" 0 0))
  (Variables|Default|SetEnemy _returnvalue_3))

(fn DrawCards
  (params (Amount :type Integer))
  (Utilities|FlowControl|ForLoopwithBreak 1 Amount :!label _label
    (:LoopBody
      ;[0.15 0 0 0.502] [TEMP] 남은 덱 크기 확인
      (if true
        ;[0.15 0.15 0.15 0.5] 카드 뽑기
        (Utilities|FlowControl|Sequence
          (:then_0
            (bind _asbp_witch (Utilities|Casting|CastToBP_Witch (Variables|Default|GetPlayer))
              (:then
                (Default|DrawCard _asbp_witch))
              (:CastFailed
                (goto _label Break))))
          (:then_1
            (bind _asbp_witch_2 (Utilities|Casting|CastToBP_Witch (Variables|Default|GetEnemy))
              (:then
                (Default|DrawCard _asbp_witch_2))
              (:CastFailed
                (goto _label Break)))))
        (else
          (goto _label Break))))))